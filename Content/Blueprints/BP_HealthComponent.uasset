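; BP_HealthComponent is an actor component that tracks replicated health with damage, healing and a death check.
; ApplyDamage and Heal clamp CurrentHealth between zero and MaxHealth, with ApplyDamage also broadcasting OnHealthChanged directly.
; The CurrentHealth RepNotify broadcasts health changes and fires OnDeath at zero.
; Debug prints report damage and snapshot every third-person character's health from the RepNotify and on authority heals.
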(fn `ApplyDamage`
  (params (Damage :type "Float (double-precision)"))
  (bind _output_get (set `self.CurrentHealth` (`KismetMathLibrary.FClamp` (- (`self.CurrentHealth`) Damage) 0.0 (`self.MaxHealth`))))
  (`self.OnHealthChanged` _output_get)
  (`KismetSystemLibrary.PrintString` (`KismetStringLibrary.Concat_StrStr` (`KismetSystemLibrary.GetDisplayName` (`self.GetOwner`)) " " "Was Damaged, and now has Current Health: " (`KismetStringLibrary.Conv_DoubleToString` (`self.CurrentHealth`))) true true (struct :`G` 0.66 :`B` 1.0 :`A` 1.0) 10.0))

(fn `DebugHealthChangedValues`
  (`KismetSystemLibrary.PrintString` "++++++++++HEALTHSNAPSHOT++++++++++" true true (struct :`G` 1.0 :`B` 0.267454 :`A` 1.0) 10.0)
  (bind _outactors (`GameplayStatics.GetAllActorsOfClass` "/Game/ThirdPerson/Blueprints/BP_ThirdPersonCharacter.BP_ThirdPersonCharacter_C"))
  (for _array_element _outactors
    (`KismetSystemLibrary.PrintString` (`KismetStringLibrary.Concat_StrStr` (`KismetSystemLibrary.GetDisplayName` _array_element) " " " Current Health: " (`KismetStringLibrary.Conv_DoubleToString` (`/Game/Blueprints/BP_HealthComponent.CurrentHealth` (`Actor.GetComponentByClass` _array_element "BP_HealthComponent_C")))) true true (struct :`G` 0.66 :`B` 1.0 :`A` 1.0) 10.0)))

(fn `Heal`
  (params (HealAmount :type "Float (double-precision)"))
  (set `self.CurrentHealth` (`KismetMathLibrary.FClamp` (+ (`self.CurrentHealth`) HealAmount) 0.0 (`self.MaxHealth`)))
  (`/Engine/EditorBlueprintResources/ActorComponentMacros.Switch Has Authority`
    (:`Authority`
      (`self.DebugHealthChangedValues`))))

(fn `IsDead`
  (returns (IsDead :type Boolean))
  (return (<= (`self.CurrentHealth`) 0.0)))

(fn `OnRep_CurrentHealth`
  (`self.OnHealthChanged` (`self.CurrentHealth`))
  (`self.DebugHealthChangedValues`)
  (if (`self.IsDead`)
    (`self.OnDeath`)))