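; Spike trap actor that damages any overlapping actor with a health component, applying damage only on the authority.
; An overlap while active triggers damage and a timeline that lowers the spikes, with an event track disarming them.
; After a delay it retries on a timer until no third-person character overlaps, then shakes the base while raising the spikes, re-arming when finished.
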(event `self.ReceiveBeginPlay`
  (bind _returnvalue_location (`KismetMathLibrary.BreakTransform` (`SceneComponent.GetRelativeTransform` (`self.Spikes_Root`))))
  (set `self.BaseStartLocation` (`self.K2_GetActorLocation`))
  (set `self.SpikeStartLocation` _returnvalue_location))

(event `self.Box_Collision.OnComponentBeginOverlap`
  (params (OverlappedComponent :type "PrimitiveComponent Object Reference") (OtherActor :type "Actor Object Reference") (OtherComp :type "PrimitiveComponent Object Reference") (OtherBodyIndex :type Integer) (bFromSweep :type Boolean) (SweepResult :type "HitResult Structure (by ref)"))
  (if (`self.IsSpikeActive`)
    (`self.ApplyDamageToHealthComponent` OtherActor)
    (bind (_direction _down) (`Timeline|TL_LowerSpikes` :!via `PlayFromStart`)
      (:`Update`
        (`SceneComponent.K2_SetRelativeLocation` (`self.Spikes_Root`) (`self.LerpSpikeLowered` _down (`self.SpikeHeightToLowerOrRaise`)) false false))
      (:`Finished`
        (`KismetSystemLibrary.K2_SetTimerDelegate` (delegate `TryRaiseSpikes`) (`self.DelayTime`)))
      (:`SpikeInactive`
        (set `self.IsSpikeActive` false)))))

(event `TryRaiseSpikes`
  (if (== (`KismetArrayLibrary.Array_Length` (`PrimitiveComponent.GetOverlappingActors` (`self.Box_Collision`) "/Game/ThirdPerson/Blueprints/BP_ThirdPersonCharacter.BP_ThirdPersonCharacter_C")) 0)
    (bind (_direction _rise _shake) (`Timeline|TL_RaiseSpike` :!via `PlayFromStart`)
      (:`Update`
        (`SceneComponent.K2_SetRelativeLocation` (`self.Base`) (+ (`self.BaseStartLocation`) (`KismetMathLibrary.MakeVector` 0.0 0.0 _shake)) false false)
        (`SceneComponent.K2_SetRelativeLocation` (`self.Spikes_Root`) (`self.LerpSpikeRaised` _rise (`self.SpikeHeightToLowerOrRaise`)) false false))
      (:`Finished`
        (set `self.IsSpikeActive` true)))
    (else
      (`KismetSystemLibrary.K2_SetTimerDelegate` (delegate `TryRaiseSpikes`) (`self.DelayTime`)))))

(fn `ApplyDamageToHealthComponent`
  (params (OtherActor :type "Actor Object Reference"))
  (bind _returnvalue (`self.GetComponentByClass` OtherActor "/Game/Blueprints/BP_HealthComponent.BP_HealthComponent_C"))
  (if (`self.IsSpikeActive`)
    (`/Engine/EditorBlueprintResources/ActorMacros.Switch Has Authority`
      (:`Authority`
        (`/Engine/EditorBlueprintResources/StandardMacros.IsValid` _returnvalue
          (:`Is Valid`
            (`/Game/Blueprints/BP_HealthComponent.ApplyDamage` _returnvalue (`self.DamageAmount`))))))))

(fn `LerpSpikeLowered`
  (params (Alpha :type "Float (single-precision)") (SpikeHeight :type "Float (double-precision)"))
  (returns (LerpValue :type "Vector Structure"))
  (return (`KismetMathLibrary.VLerp` (`self.SpikeStartLocation`) (- (`self.SpikeStartLocation`) (`KismetMathLibrary.MakeVector` 0.0 0.0 SpikeHeight)) Alpha)))

(fn `LerpSpikeRaised`
  (params (Alpha :type "Float (single-precision)") (SpikeHeight :type "Float (double-precision)"))
  (returns (LerpValue :type "Vector Structure"))
  (return (`KismetMathLibrary.VLerp` (- (`self.SpikeStartLocation`) (`KismetMathLibrary.MakeVector` 0.0 0.0 SpikeHeight)) (`self.SpikeStartLocation`) Alpha)))

(fn `UserConstructionScript`)